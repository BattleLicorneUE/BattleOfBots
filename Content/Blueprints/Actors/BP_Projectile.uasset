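; Projectile actor fired by a bot that deals point damage to characters it hits and destroys itself on any hit.
; The sphere's hit event damages any character other than the owning RefBot, crediting that bot as causer and its controller as instigator.
; Damaged characters and non-character impacts get separate sounds but share one Niagara effect, while hitting the owner gives neither damage nor feedback.
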(event `self.Sphere.OnComponentHit`
  (params (HitComponent :type "PrimitiveComponent Object Reference") (OtherActor :type "Actor Object Reference") (OtherComp :type "PrimitiveComponent Object Reference") (NormalImpulse :type "Vector Structure") (Hit :type "HitResult Structure (by ref)"))
  (bind _ascharacter (cast `Character` OtherActor)
    (:`then`
      (`self.Apply Damages` _ascharacter Hit))
    (:`CastFailed`
      (`self.play Feelback` (`.Location` (`GameplayStatics.BreakHitResult` Hit)) "/Game/SFX/Gun/SoundCue_Hit.SoundCue_Hit" "/Game/VFX/NS_Hit_Player.NS_Hit_Player")))
  (`self.K2_DestroyActor`))

(fn `Apply Damages`
  (params (Object :type "Actor Object Reference") (HitInfo :type "HitResult Structure (by ref)"))
  (bind (_bblockinghit _binitialoverlap _time _distance _location _impactpoint _normal _impactnormal _physmat _hitactor _hitcomponent _hitbonename _bonename _hititem _elementindex _faceindex _tracestart) (`GameplayStatics.BreakHitResult` HitInfo))
  (bind _ref_bot_ (`self.Ref Bot `))
  (if (not (== Object _ref_bot_))
    (`GameplayStatics.ApplyPointDamage` Object 20.0 _tracestart HitInfo (`self.GetInstigatorController` _ref_bot_) _ref_bot_)
    (`self.play Feelback` _location "/Game/SFX/Gun/SoundCue_HitCharacter.SoundCue_HitCharacter" "/Game/VFX/NS_Hit_Player.NS_Hit_Player")
    (return)))

(fn `OnRep_Ref Bot `)

(fn `play Feelback`
  (params (Location :type "Vector Structure") (Sound :type "SoundBase Object Reference") (SystemTemplate :type "NiagaraSystem Object Reference"))
  (`GameplayStatics.PlaySoundAtLocation` Sound Location (struct) 1.0 1.0 0.0 null null null null)
  (`NiagaraFunctionLibrary.SpawnSystemAtLocation` SystemTemplate Location))

(fn `UserConstructionScript`)