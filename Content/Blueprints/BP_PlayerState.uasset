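; BP_PlayerState tracks a player's score, kills, deaths and kill/death ratio.
; AddScoring awards a fixed score increment, while AddKill and AddDeath increase their counters and then call CalculateRatio.
; CalculateRatio uses SelectFloat to divide by one when there are no deaths, avoiding division by zero, and prints the result with PrintString.
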(fn `Add Death`
  (set `self.Death` (+ (`self.Death`) 1.0))
  (`self.Calculate Ratio`))

(fn `Add Kill`
  (set `self.Kill` (+ (`self.Kill`) 1.0))
  (`self.Calculate Ratio`))

(fn `Add Scoring`
  (set `self.Scoring` (+ (`self.Scoring`) 100)))

(fn `Calculate Ratio`
  (bind _death (`self.Death`))
  (bind _output_get (set `self.Ratio` (/ (`self.Kill`) (`KismetMathLibrary.SelectFloat` 1.0 _death (<= _death 0.0)))))
  (`KismetSystemLibrary.PrintString` (`KismetStringLibrary.Conv_DoubleToString` _output_get))
  (return))

(fn `UserConstructionScript`)